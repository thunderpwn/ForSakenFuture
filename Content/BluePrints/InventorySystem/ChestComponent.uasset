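; Chest inventory component that stores items in a fixed number of slots and toggles a chest window on the player's HUD.
; PrepareChest sizes the array and refreshes slot data from item class defaults on BeginPlay and before the window opens.
; AddToChest fills partial stacks first, with overflow recursing through AddToStack, otherwise CreateStack takes an empty slot.
; ChestQuery totals an item class against a requested amount; unused backpack-window logic remains.
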(event EventBeginPlay
  (CallFunction|PrepareChest))

(event EventTick
  (params (DeltaSeconds :type Float%20%28single-precision%29)))

(fn ToggleChest
  (bind _returnvalue (Game|GetPlayerController 0))
  (bind _returnvalue_2 (Game|GetPlayerController 0))
  (bind _self self)
  (Variables|Default|GetChestWindow
    (:then
      (Widget|RemovefromParent (Variables|Default|GetChestWindow))
      (Variables|Default|SetChestWindow 0)
      (Input|SetInputModeGameOnly _returnvalue_2)
      (Variables|/Script/Engine.PlayerController|SetbShowMouseCursor _returnvalue_2 false))
    (:else
      (CallFunction|PrepareChest)
      (bind _returnvalue_3 (UserInterface|CreateWidget "/Game/BluePrints/InventorySystem/InventoryUI/ChestWindow.ChestWindow_C" 0 _self (Variables|Default|GetInventoryName _self)))
      (Variables|Default|SetChestWindow _returnvalue_3)
      (bind _asff_player_controller (Utilities|Casting|CastToFF_PlayerController (Game|GetPlayerController 0)))
      (bind _returnvalue_4 (Class|CanvasPanel|AddChildtoCanvas (Variables|/Game/Ui/Ingame/InGameHud.InGameHud_C|GetHudCanvas (Variables|/Game/BluePrints/Game/FF_PlayerController.FF_PlayerController_C|GetIngameHud _asff_player_controller)) (Variables|Default|GetChestWindow)))
      (Class|CanvasPanelSlot|SetAutoSize _returnvalue_4 true)
      (Input|SetInputModeUIOnly _returnvalue (Variables|Default|GetChestWindow) "LockAlways")
      (Variables|/Script/Engine.PlayerController|SetbShowMouseCursor _returnvalue true))))

(fn AddtoChest
  (params (ContentToAdd :type Slot%20Structure%20Structure))
  (if (.isstackable? (.itemstructure ContentToAdd))
    (bind _stackindex (Utilities|HasPartialStack ContentToAdd)
      (:True
        (bind _sucsess (CallFunction|AddtoStack ContentToAdd _stackindex))
        (if _sucsess
          _
          (else
            (Development|PrintString "doesnt work on partial")
            (return false))))
      (:False
        (bind _sucsess_2 (CallFunction|CreateStack ContentToAdd :!label _label))
        (if _sucsess_2
          _
          (else
            (Development|PrintString "cant seem to add")
            (return false)))))
    (else
      (goto _label)))
  (return true))

(fn PrepareChest
  (bind _inventory (Variables|Default|GetInventory))
  (Utilities|Array|Resize (Variables|Default|GetInventory) (Variables|Default|GetNumberOfSlots))
  (for (_array_element _array_index) (Variables|Default|GetInventory)
    (if (< (.quantity _array_element) 1)
      (bind _structout (Utilities|Struct|SetmembersinSlotStructure (Utilities|Array|Get(acopy) (Variables|Default|GetInventory) _array_index) (Utilities|Struct|MakeItemStructure "" false 0 4 true "" 0.0 1e+01 0.0 false "NewEnumerator0" false "NewEnumerator3" 0)))
      (Utilities|Array|SetArrayElem _inventory _array_index _structout)
      (elif (!= (.Class (Utilities|Struct|BreakItemStructure (.itemstructure _array_element))) 0)
        (Utilities|Array|SetArrayElem _inventory _array_index (Utilities|Struct|MakeSlotStructure (Utilities|GetClassDefaults (.Class (Utilities|Struct|BreakItemStructure (.itemstructure _array_element)))) (.quantity _array_element)))))))

(fn CreateStack
  (params (ContentToAdd :type Slot%20Structure%20Structure))
  (bind (_array_element _array_index) (Utilities|Array|ForEachLoopwithBreak (Variables|Default|GetInventory) :!label _label)
    (:LoopBody
      (if (<= (.quantity _array_element) 0)
        (LocalVariables|SetHasSpace? true)
        (goto _label Break)))
    (:Completed
      (if (LocalVariables|GetHasSpace?)
        (Utilities|Array|SetArrayElem (Variables|Default|GetInventory) _array_index ContentToAdd)
        (return (LocalVariables|GetHasSpace?))
        (else
          (return false))))))

(fn AddtoStack
  (params (SlotStructure :type Slot%20Structure%20Structure) (SlotIndex :type Integer))
  (bind _inventory (Variables|Default|GetInventory))
  (bind _inventory_2 (Variables|Default|GetInventory))
  (bind _maxstacksize (Utilities|Struct|BreakItemStructure (.itemstructure SlotStructure)))
  (bind _output (Utilities|Array|Get(acopy) _inventory SlotIndex))
  (bind _output_2 (Utilities|Array|Get(acopy) _inventory_2 SlotIndex))
  (bind _output_get (LocalVariables|SetCurrentQuantity (.quantity _output)))
  (if (> (+ _output_get (.Quantity (Utilities|Struct|BreakSlotStructure SlotStructure))) (.maxstacksize (.itemstructure _output)))
    (Utilities|Array|SetArrayElem (Variables|Default|GetInventory) SlotIndex (Utilities|Struct|MakeSlotStructure (.itemstructure SlotStructure) _maxstacksize))
    (CallFunction|AddtoChest (Utilities|Struct|MakeSlotStructure (.itemstructure SlotStructure) (- (.quantity SlotStructure) (- _maxstacksize (LocalVariables|GetCurrentQuantity)))))
    (else
      (Utilities|Array|SetArrayElem _inventory_2 SlotIndex (Utilities|Struct|MakeSlotStructure (.itemstructure _output_2) (+ (.quantity SlotStructure) (.quantity _output_2))))))
  (return true))

(fn ChestQuery
  (params (ItemClass :type Item%20Class%20Reference) (QueryAmount :type Integer))
  (bind _array_element (Utilities|Array|ForEachLoopwithBreak (Variables|Default|GetInventory))
    (:LoopBody
      (if (== (.Class (Utilities|Struct|BreakItemStructure (.itemstructure _array_element))) ItemClass)
        (LocalVariables|SetRunningTotal (+ (.quantity _array_element) (LocalVariables|GetRunningTotal)))))
    (:Completed
      (if (>= QueryAmount (LocalVariables|GetRunningTotal))
        (return true)
        (else
          (return false))))))