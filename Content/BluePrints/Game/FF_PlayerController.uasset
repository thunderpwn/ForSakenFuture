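; Multiplayer player controller that handles a player's HUD, in-game menu, chat and saved profile.
; BeginPlay creates the HUD, while M toggles the menu and T toggles chat input by switching cursor and input mode.
; InitialSetup loads player settings from a save slot, then has WorldGameMode respawn the player and update everyone.
; Chat messages are relayed to every controller in the game mode's list, and EndPlay returns to the main menu through FF_GameInstance.
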(event Custom|GetChatMessage
  (params (TextToSend :type Text))
  ;[1 1 1] Chat Related
  (Variables|Chat|SetSenderText TextToSend)
  (Variables|Chat|SetSenderName (.PlayerName (Utilities|Struct|BreakPlayerInfo (Variables|PlayerInfo|GetPlayerSettings))))
  (bind _asworld_game_mode (Utilities|Casting|CastToWorldGameMode (Game|GetGameMode)))
  (for _array_element (Variables|/Game/BluePrints/Game/WorldGameMode.WorldGameMode_C|GetAllPlayerControllers _asworld_game_mode)
    (bind _asff_player_controller (Utilities|Casting|CastToFF_PlayerController _array_element))
    (CallFunction|UpdateChat _asff_player_controller (Utilities|Text|ToText(String) (Variables|Chat|GetSenderName)) (Variables|Chat|GetSenderText))))

(event Custom|UpdateChat
  (params (Sender :type Text) (Text :type Text))
  ;[1 1 1] Chat Related
  (Default|UpdateChatWindow (Variables|/Game/Ui/Ingame/InGameHud.InGameHud_C|GetChatWindow (Variables|Default|GetIngameHud)) Sender Text))

(event Custom|InitialSetup
  ;[1 1 1] Initial setup- check for savegame and tell server to update
  (CallFunction|SaveGameCheck)
  (CallFunction|CallUpdate (Variables|PlayerInfo|GetPlayerSettings)))

(event Custom|CallUpdate
  (params (Playerinfo :type Player%20Info%20Structure))
  (bind _returnvalue (Game|GetGameMode))
  (bind (_asworld_game_mode _bsuccess) (Utilities|Casting|CastToWorldGameMode _returnvalue))
  ;[1 1 1] Tells everyone to update new player
  (Variables|PlayerInfo|SetPlayerSettings Playerinfo)
  (Default|RespawnPlayer _asworld_game_mode self)
  (Default|EveryOneUpdate _asworld_game_mode)
  (Development|PrintString (Utilities|String|ToString(Boolean) _bsuccess)))

(event Custom|AddPlayerInfo
  (params (AllPlayerInfos :type Array%20of%20Player%20Info%20Structures))
  ;[1 1 1] Update Playerlist window
  (Variables|PlayerInfo|SetAllConnectedPlayers AllPlayerInfos)
  (Utilities|IsValid 0))

(event Custom|UpdateNumberOfPlayers
  (params (CurrentPlayers :type Integer) (MaxPlayers :type Integer))
  ;[1 1 1] UpdatePlayerList
)

(event EventBeginPlay
  ;[1 1 1] Init playercontroller and set gender chosen and name
  (bind _returnvalue (UserInterface|CreateWidget "/Game/Ui/Ingame/InGameHud.InGameHud_C" (Game|GetPlayerController 0)))
  (bind _output_get (Variables|Default|SetIngameHud _returnvalue))
  (UserInterface|Viewport|AddtoViewport _output_get 0))

(event EventTick
  (params (DeltaSeconds :type Float%20%28single-precision%29)))

(event EventEndPlay
  (params (EndPlayReason :type EEndPlayReason%20Enum :default "Destroyed"))
  ;[1 1 1] if session suddenly fails or server quits
  (bind _asff_game_instance (Utilities|Casting|CastToFF_GameInstance (Game|GetGameInstance)))
  (Default|QuittoMenu _asff_game_instance self))

(event Input|KeyboardEvents|M
  (params (Key :type Key%20Structure :default "None"))
  (bind _self self)
  ;[1 1 1] Press M for IngameMenu
  (:Pressed
    (if (Variables|IngameMenu|GetShowMenu?)
      (Variables|IngameMenu|SetShowMenu? false)
      (Variables|Default|SetbShowMouseCursor false)
      (Input|SetInputModeGameOnly _self)
      (else
        (Variables|IngameMenu|SetShowMenu? true)
        (Variables|Default|SetbShowMouseCursor true)
        (bind _returnvalue (UserInterface|CreateWidget "/Game/Ui/Ingame/IngameMenu.IngameMenu_C" _self))
        (Input|SetInputModeGameandUI self _returnvalue "LockOnCapture" true)))))

(event Input|KeyboardEvents|T
  (params (Key :type Key%20Structure :default "None"))
  ;[1 1 1] toggle T to text messages
  (:Pressed
    (if (Variables|Default|GetbShowMouseCursor)
      (Variables|Default|SetbShowMouseCursor false)
      (Input|SetInputModeGameOnly self)
      (else
        (Variables|Default|SetbShowMouseCursor true)
        (Input|SetInputModeGameandUI self (Variables|Default|GetIngameHud) "DoNotLock" true)))))

(fn ConstructionScript)

(fn SaveGameCheck
  (bind _returnvalue (SaveGame|DoesSaveGameExist (Variables|Default|GetFF_SaveGame)))
  (if _returnvalue
    (CallFunction|LoadGame)))

(fn LoadGame
  (bind _returnvalue (SaveGame|LoadGamefromSlot (Variables|Default|GetFF_SaveGame)))
  (bind _asff_save_game (Utilities|Casting|CastToFF_SaveGame _returnvalue))
  (Utilities|Struct|SetmembersinPlayerInfo (Variables|PlayerInfo|GetPlayerSettings) (.PlayerName (Utilities|Struct|BreakPlayerInfo (Variables|/Game/BluePrints/All/FF_SaveGame.FF_SaveGame_C|GetSaved_PlayerInfo _asff_save_game))) (.PlayerScore (Utilities|Struct|BreakPlayerInfo (Variables|/Game/BluePrints/All/FF_SaveGame.FF_SaveGame_C|GetSaved_PlayerInfo _asff_save_game))) (.PlayersLevel (Utilities|Struct|BreakPlayerInfo (Variables|/Game/BluePrints/All/FF_SaveGame.FF_SaveGame_C|GetSaved_PlayerInfo _asff_save_game))) (.PlayersChosenGender (Utilities|Struct|BreakPlayerInfo (Variables|/Game/BluePrints/All/FF_SaveGame.FF_SaveGame_C|GetSaved_PlayerInfo _asff_save_game))) (.PlayersChosenTeam (Utilities|Struct|BreakPlayerInfo (Variables|/Game/BluePrints/All/FF_SaveGame.FF_SaveGame_C|GetSaved_PlayerInfo _asff_save_game)))))

(fn SaveGame
  (Utilities|IsValid (Variables|Default|GetSaveGameRef)
    (:Is%20Valid
      _)
    (:Is%20Not%20Valid
      (bind _returnvalue (SaveGame|CreateSaveGameObject "/Script/Engine.SaveGame"))
      (bind _asff_save_game (Utilities|Casting|CastToFF_SaveGame _returnvalue))
      (bind _output_get (Variables|Default|SetSaveGameRef _asff_save_game))))
  (Variables|/Game/BluePrints/All/FF_SaveGame.FF_SaveGame_C|SetSaved_PlayerInfo _output_get (Variables|PlayerInfo|GetPlayerSettings))
  (SaveGame|SaveGametoSlot _output_get (Variables|Default|GetFF_SaveGame)))